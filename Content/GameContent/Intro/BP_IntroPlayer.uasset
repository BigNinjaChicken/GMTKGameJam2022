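; BP_IntroPlayer is the player Blueprint for a level intro, showing a moving image before loading the next level.
; On BeginPlay it plays menu music, then a timeline slides the PlayerIntroImage actor to the DiceIntro's GoTo point while Tick keeps the camera aimed at it.
; When the timeline ends, it increments the saved level in GI_SavedData and opens that level, or the menu past the last.
; LeaveGame input quits.
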(event EventBeginPlay
  (Utilities|FlowControl|Sequence
    (:then_0
      (bind _returnvalue (Actor|GetActorOfClass "/Game/GameContent/Intro/PlayerIntroImage.PlayerIntroImage_C"))
      (Variables|Default|SetIntroImage _returnvalue))
    (:then_1
      (bind _returnvalue_2 (Actor|GetActorOfClass "/Game/GameContent/Intro/DiceIntro.DiceIntro_C"))
      (Variables|Default|SetDiceIntro _returnvalue_2))
    (:then_2
      (Audio|PlaySound2D "/Game/GameContent/Menu/415805__sunsai__menu-background-music.415805__sunsai__menu-background-music" 1.0 1.0 0.0 0 0))
    (:then_3
      (Utilities|FlowControl|Delay 1.0)
      (Variables|Default|SetNewVar_0 (Transformation|GetActorLocation (Variables|Default|GetIntroImage)))
      (Variables|Default|SetNewVar_1 (Transformation|GetWorldLocation (Variables|/Game/GameContent/Intro/DiceIntro.DiceIntro_C|GetGoTo (Variables|Default|GetDiceIntro))))
      (Components|Timeline|SetPlayRate (Variables|Default|GetIntroTimeline) 0.2)
      (bind _speed (Timeline|IntroTimeline PlayFromStart)
        (:Update
          (Transformation|SetActorLocation (Variables|Default|GetIntroImage) (Math|Vector|Lerp(Vector) (Variables|Default|GetNewVar_0) (Variables|Default|GetNewVar_1) _speed) false false))
        (:Finished
          (bind _asgi_saved_data (Utilities|Casting|CastToGI_SavedData (Game|GetGameInstance)))
          (bind _result (Math|Integer|IncrementInt (Variables|/Game/GameContent/GI_SavedData.GI_SavedData_C|GetCurrentLevel _asgi_saved_data))
            (:%20%20
              (if (> _result (Variables|/Game/GameContent/GI_SavedData.GI_SavedData_C|GetTotalLevels _asgi_saved_data))
                (Game|OpenLevel(byName) "LV_Menu")
                (else
                  (Game|OpenLevel(byName) (Utilities|String|StringToName (Utilities|String|Append (Variables|Default|GetLV_Level) (Utilities|String|ToString(Integer) (Variables|/Game/GameContent/GI_SavedData.GI_SavedData_C|GetCurrentLevel _asgi_saved_data))))))))))))))

(event EventTick
  (params (DeltaSeconds :type Float%20%28single-precision%29))
  (bind _camera (Variables|Default|GetCamera))
  (bind _introimage (Variables|Default|GetIntroImage))
  (bind _returnvalue (Transformation|GetActorLocation _introimage))
  (bind _returnvalue_2 (Transformation|GetWorldLocation _camera))
  (bind _returnvalue_3 (Math|Rotator|FindLookatRotation _returnvalue_2 _returnvalue))
  (Transformation|SetWorldRotation (Variables|Default|GetCamera) (Math|Interpolation|RInterpTo (Transformation|GetWorldRotation (Variables|Default|GetCamera)) (Math|Rotator|MakeRotator (.roll _returnvalue_3) (.pitch _returnvalue_3) (.yaw _returnvalue_3)) DeltaSeconds 0.0) false false))

(event Input|ActionEvents|InputActionLeaveGame
  (params (Key :type Key%20Structure :default "None"))
  (:Pressed
    (Game|QuitGame 0 "Quit" false)))

(fn ConstructionScript)