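; BP_MenuPlayer is the player Blueprint for the menu, setting up the menu screen and handling quitting.
; On BeginPlay it adds WBP_Menu to the viewport, plays 2D background music, and passes CurrentTime from the GI_SavedData game instance to the widget's Time text.
; Pressing the LeaveGame input action quits the game.
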(event EventBeginPlay
  (Utilities|FlowControl|Sequence
    (:then_0
      (bind _returnvalue (UserInterface|CreateWidget "/Game/GameContent/Menu/WBP_Menu.WBP_Menu_C"))
      (bind _output_get (Variables|Default|SetUI _returnvalue))
      (UserInterface|Viewport|AddtoViewport _output_get 0))
    (:then_1
      (Audio|PlaySound2D "/Game/GameContent/Menu/415805__sunsai__menu-background-music.415805__sunsai__menu-background-music" 1.0 1.0 0.0 0 0))
    (:then_2
      (bind _asgi_saved_data (Utilities|Casting|CastToGI_SavedData (Game|GetGameInstance)))
      (Variables|/Game/GameContent/Menu/WBP_Menu.WBP_Menu_C|SetTime (Variables|Default|GetUI) (Utilities|Text|ToText(Float) (Variables|/Game/GameContent/GI_SavedData.GI_SavedData_C|GetCurrentTime _asgi_saved_data) "HalfToEven")))))

(event Collision|EventActorBeginOverlap
  (params (OtherActor :type Actor%20Object%20Reference)))

(event EventTick
  (params (DeltaSeconds :type Float%20%28single-precision%29)))

(event Input|ActionEvents|InputActionLeaveGame
  (params (Key :type Key%20Structure :default "None"))
  (:Pressed
    (Game|QuitGame 0 "Quit" false)))

(fn ConstructionScript)