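; BP_Player2 is a player Blueprint with mouse look and unfinished physics-based movement.
; Mouse axes yaw PlayerHitBox and pitch Camera, scaled by sensitivity.
; Both movement axes share one path that stops horizontal velocity when grounded without input, using GroundCheck overlaps.
; Otherwise, below MoveSpeed on X or Y, it prints the intended movement vector but applies zero force.
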(event Input|AxisEvents|InputAxisRotateMouseX
  (params (AxisValue :type Float%20%28single-precision%29))
  (Transformation|AddLocalRotation (Variables|Default|GetPlayerHitBox) (Math|Rotator|MakeRotator 0.0 0.0 (* AxisValue (Variables|Default|GetXSensitivity))) false false))

(event Input|AxisEvents|InputAxisRotateMouseY
  (params (AxisValue :type Float%20%28single-precision%29))
  (Transformation|AddLocalRotation (Variables|Default|GetCamera) (Math|Rotator|MakeRotator 0.0 (* AxisValue (Variables|Default|GetYSensitivity)) 0.0) false false))

(event Input|AxisEvents|InputAxisMoveLeftRight
  (params (AxisValue :type Float%20%28single-precision%29))
  (bind _playerhitbox (Variables|Default|GetPlayerHitBox))
  (bind _movespeed (Variables|Default|GetMoveSpeed))
  (bind _playerhitbox_2 (Variables|Default|GetPlayerHitBox))
  (bind _returnvalue (Transformation|GetComponentVelocity _playerhitbox_2))
  (bind _output_get (Variables|Default|SetMoveVector (Math|Vector|MakeVector (stale Input|AxisEvents|InputAxisMoveForwardBackward AxisValue) AxisValue 0.0)))
  (bind _grounded (CallFunction|IsGrounded))
  (if (and _grounded (Utilities|Operators|EqualEqual :A (Math|Vector|Normalize _output_get) :ErrorTolerance 0.0))
    (Physics|SetPhysicsLinearVelocity _playerhitbox (Math|Vector|MakeVector 0.0 0.0 (.z (Transformation|GetComponentVelocity _playerhitbox))) false "None")
    (elif (or (< (.x _returnvalue) _movespeed) (< (.y _returnvalue) _movespeed))
      (Development|PrintString (Utilities|String|ToString(Vector) (* (Math|Vector|Normalize _output_get) (Variables|Default|GetMoveSpeed))))
      (Physics|AddForce (Variables|Default|GetPlayerHitBox) "0, 0, 0" "None" false))))

(event Input|AxisEvents|InputAxisMoveForwardBackward
  (params (AxisValue :type Float%20%28single-precision%29))
  (bind _playerhitbox (Variables|Default|GetPlayerHitBox))
  (bind _movespeed (Variables|Default|GetMoveSpeed))
  (bind _playerhitbox_2 (Variables|Default|GetPlayerHitBox))
  (bind _returnvalue (Transformation|GetComponentVelocity _playerhitbox_2))
  (bind _output_get (Variables|Default|SetMoveVector (Math|Vector|MakeVector AxisValue (stale Input|AxisEvents|InputAxisMoveLeftRight AxisValue) 0.0)))
  (bind _grounded (CallFunction|IsGrounded))
  (if (and _grounded (Utilities|Operators|EqualEqual :A (Math|Vector|Normalize _output_get) :ErrorTolerance 0.0))
    (Physics|SetPhysicsLinearVelocity _playerhitbox (Math|Vector|MakeVector 0.0 0.0 (.z (Transformation|GetComponentVelocity _playerhitbox))) false "None")
    (elif (or (< (.x _returnvalue) _movespeed) (< (.y _returnvalue) _movespeed))
      (Development|PrintString (Utilities|String|ToString(Vector) (* (Math|Vector|Normalize _output_get) (Variables|Default|GetMoveSpeed))))
      (Physics|AddForce (Variables|Default|GetPlayerHitBox) "0, 0, 0" "None" false))))

(fn ConstructionScript)

(fn IsGrounded
  (return (> (Utilities|Array|Length (Collision|GetOverlappingActors (Variables|Default|GetGroundCheck) 0 :!class /Script/Engine.PrimitiveComponent)) 1)))