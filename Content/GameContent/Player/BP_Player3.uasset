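; Player character with camera-relative movement, mouse look, a dash and a sword attack.
; Dash lerps the capsule to the DashPoint or first traced hit via timeline, suspending gravity and walk speed, then jumps and restores both.
; Attack plays a slice sequence and damages BP_EnemyParent actors overlapping SwordHitBox; both abilities shake the camera.
; DoOnce gates reset by timelines provide cooldowns, though the sword cooldown sets EndDashTimer's rate, not its own.
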(event Custom|EndDash
  (params (DashCoolDown :type Boolean))
  (bind _charactermovement (Variables|Character|GetCharacterMovement))
  (Components|Timeline|SetPlayRate (Variables|Default|GetEndDashTimer) (/ 1.0 (Variables|Default|GetDashCoolDown)))
  (bind _speed (Timeline|EndDashTimer PlayFromStart)
    (:Finished
      (Utilities|FlowControl|DoOnce false) ; enters at Reset
    )))

(event Custom|StartSwordCooldown
  (bind _swordslicesequence (Variables|Default|GetSwordSliceSequence))
  (bind _sequenceplayer (Variables|/Script/ActorSequence.ActorSequenceComponent|GetSequencePlayer _swordslicesequence))
  (Components|Timeline|SetPlayRate (Variables|Default|GetEndDashTimer) (/ 1.0 (Variables|Default|GetSwordCooldown)))
  (bind _speed (Timeline|SwordCooldownTimeline PlayFromStart)
    (:Finished
      (Utilities|FlowControl|DoOnce false) ; enters at Reset
    )))

(event EventBeginPlay
  (Variables|Default|SetCharacterWalkSpeed (Variables|/Script/Engine.CharacterMovementComponent|GetMaxWalkSpeed (Variables|Character|GetCharacterMovement))))

(event Input|ActionEvents|InputActionDash
  (params (Key :type Key%20Structure :default "None"))
  (bind _charactermovement (Variables|Character|GetCharacterMovement))
  (:Pressed
    (Utilities|FlowControl|DoOnce false
      (:Completed
        (Variables|/Script/Engine.CharacterMovementComponent|SetGravityScale _charactermovement 0.0)
        (Variables|/Script/Engine.CharacterMovementComponent|SetMaxWalkSpeed _charactermovement 0.0)
        (Variables|Default|SetStartDashLocation (Transformation|GetWorldLocation (Variables|Collision|GetCapsuleComponent)))
        (Variables|Default|SetEndDastLocation (Transformation|GetWorldLocation (Variables|Default|GetDashPoint)))
        (bind (_outhit _returnvalue) (Collision|LineTraceByChannel (Variables|Default|GetStartDashLocation) (Variables|Default|GetEndDastLocation) "TraceTypeQuery1" false 0 "Persistent"))
        (if _returnvalue
          (Variables|Default|SetEndDastLocation (.Location (Collision|BreakHitResult _outhit))))
        (Components|Timeline|SetPlayRate (Variables|Default|GetDash) 3.0)
        (bind _speed (Timeline|Dash PlayFromStart)
          (:Update
            (Transformation|SetWorldLocation (Variables|Collision|GetCapsuleComponent) (Math|Vector|Lerp(Vector) (Variables|Default|GetStartDashLocation) (Variables|Default|GetEndDastLocation) _speed) false false)
            (Camera|PlayWorldCameraShake "/Game/GameContent/Player/BP_DashCamShake.BP_DashCamShake_C" (Transformation|GetActorLocation) 0.0 5e+02))
          (:Finished
            (Character|Jump)
            (CallFunction|EndDash false)
            (Components|Timeline|SetPlayRate (Variables|Default|GetDashEnd) 3.0)
            (Timeline|DashEnd PlayFromStart
              (:Update
                (Variables|/Script/Engine.CharacterMovementComponent|SetGravityScale (Variables|Character|GetCharacterMovement) 1.0)
                (Variables|/Script/Engine.CharacterMovementComponent|SetMaxWalkSpeed (Variables|Character|GetCharacterMovement) (Variables|Default|GetCharacterWalkSpeed)))
              (:Finished
                (Character|StopJumping)))))))))

(event Input|ActionEvents|InputActionAttack
  (params (Key :type Key%20Structure :default "None"))
  (bind _swordslicesequence (Variables|Default|GetSwordSliceSequence))
  (bind _sequenceplayer (Variables|/Script/ActorSequence.ActorSequenceComponent|GetSequencePlayer _swordslicesequence))
  (:Pressed
    (Utilities|FlowControl|DoOnce false
      (:Completed
        (Utilities|FlowControl|Sequence
          (:then_0
            (Components|Timeline|SetPlayRate _sequenceplayer 3.0)
            (Sequencer|Player|Play _sequenceplayer :!class /Script/MovieScene.MovieSceneSequencePlayer))
          (:then_1
            (for _array_element (Collision|GetOverlappingActors (Variables|Default|GetSwordHitBox) 0 :!class /Script/Engine.PrimitiveComponent)
              (bind _asbp_enemy_parent (Utilities|Casting|CastToBP_EnemyParent _array_element))
              (Default|TakeDamage _asbp_enemy_parent)))
          (:then_2
            (Camera|PlayWorldCameraShake "/Game/GameContent/Player/BP_SwordCamShake.BP_SwordCamShake_C" (Transformation|GetActorLocation) 0.0 5e+02))
          (:then_4
            (CallFunction|StartSwordCooldown)))))))

(event Input|AxisEvents|InputAxisRotateMouseX
  (params (AxisValue :type Float%20%28single-precision%29))
  (Pawn|Input|AddControllerYawInput AxisValue))

(event Input|AxisEvents|InputAxisRotateMouseY
  (params (AxisValue :type Float%20%28single-precision%29))
  (Pawn|Input|AddControllerPitchInput AxisValue))

(event Input|AxisEvents|InputAxisMoveForwardBackward
  (params (AxisValue :type Float%20%28single-precision%29))
  (Pawn|Input|AddMovementInput (Math|Vector|GetForwardVector (Math|Rotator|MakeRotator 0.0 0.0 (.yaw (Pawn|GetControlRotation :!class /Script/Engine.Pawn)))) AxisValue false))

(event Input|AxisEvents|InputAxisMoveLeftRight
  (params (AxisValue :type Float%20%28single-precision%29))
  (Pawn|Input|AddMovementInput (Math|Vector|GetRightVector (Math|Rotator|MakeRotator 0.0 0.0 (.yaw (Pawn|GetControlRotation :!class /Script/Engine.Pawn)))) AxisValue false))

(fn ConstructionScript)