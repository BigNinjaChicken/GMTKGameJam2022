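; Physics-driven first-draft player with mouse look, forward/back movement and an unfinished dash.
; Mouse yaw turns the hitbox and pitch turns the camera, while a MoveForward timeline ramps the impulse applied to the hitbox each Tick.
; When that timeline finishes at zero speed, an overlap-based ground check gates stopping horizontal velocity.
; Dash only sets state and runs its timeline, as its velocity logic, strafing and speed clamping are disconnected.
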(event Custom|AddMovement
  (params (DeltaSconds :type Float%20%28double-precision%29))
  (if (> (stale Input|AxisEvents|InputAxisMoveForwardBackward _speed) 0.0)
    (if true
      (Physics|AddImpulse (Variables|Default|GetPlayerHitBox) (* (Math|Vector|Normalize (Math|Vector|GetForwardVector (Variables|Default|GetPlayerHitBox))) (* (* (stale Input|AxisEvents|InputAxisMoveForwardBackward _speed) (Variables|Default|GetForwardSpeed)) (Variables|Default|GetForwardBackwardAxisValue))) "None" false))))

(event EventBeginPlay)

(event EventTick
  (params (DeltaSeconds :type Float%20%28single-precision%29))
  (Variables|Default|SetDelta%20Seconds DeltaSeconds)
  (Utilities|FlowControl|Sequence
    (:then_0
      (CallFunction|AddMovement (Variables|Default|GetDelta%20Seconds)))))

(event Input|ActionEvents|InputActionDash
  (params (Key :type Key%20Structure :default "None"))
  (:Pressed
    (Utilities|FlowControl|DoOnce false :!label _label
      (:Completed
        (Variables|Default|SetCameraForwardVector (Math|Vector|GetForwardVector (Variables|Default|GetCamera)))
        (Components|Timeline|SetPlayRate (Variables|Default|GetDashTimeLine) 1e+01)
        (Variables|Default|SetisDashing true)
        (bind _speed (Timeline|DashTimeLine PlayFromStart)
          (:Finished
            (Variables|Default|SetisDashing false))))))
  (:Released
    (goto _label Reset)))

(event Input|AxisEvents|InputAxisRotateMouseX
  (params (AxisValue :type Float%20%28single-precision%29))
  (Transformation|AddLocalRotation (Variables|Default|GetPlayerHitBox) (Math|Rotator|MakeRotator 0.0 0.0 (* AxisValue (Variables|Default|GetXSensitivity))) false false))

(event Input|AxisEvents|InputAxisRotateMouseY
  (params (AxisValue :type Float%20%28single-precision%29))
  (Transformation|AddLocalRotation (Variables|Default|GetCamera) (Math|Rotator|MakeRotator 0.0 (* AxisValue (Variables|Default|GetYSensitivity)) 0.0) false false))

(event Input|AxisEvents|InputAxisMoveLeftRight
  (params (AxisValue :type Float%20%28single-precision%29)))

(event Input|AxisEvents|InputAxisMoveForwardBackward
  (params (AxisValue :type Float%20%28single-precision%29))
  (bind _playerhitbox (Variables|Default|GetPlayerHitBox))
  (Utilities|FlowControl|Sequence
    (:then_0
      (if (> AxisValue 0.0)
        (Utilities|FlowControl|Sequence
          (:then_0
            (goto _label_3 Reset))
          (:then_1
            (Utilities|FlowControl|DoOnce false :!label _label
              (:Completed
                (Variables|Default|SetForwardBackwardAxisValue AxisValue :!label _label_2)
                (Components|Timeline|SetPlayRate (Variables|Default|GetMoveForward) (Variables|Default|GetSpeedBuildUp))
                (bind _speed (Timeline|MoveForward PlayFromStart)
                  (:Finished
                    (bind _grounded (CallFunction|IsGrounded))
                    (if (and _grounded (== _speed 0.0))
                      (Physics|SetPhysicsLinearVelocity _playerhitbox (Math|Vector|MakeVector 0.0 0.0 (.z (Transformation|GetComponentVelocity _playerhitbox))) false "None"))))))))))
    (:then_1
      (if (< AxisValue 0.0)
        (Utilities|FlowControl|Sequence
          (:then_0
            (goto _label Reset))
          (:then_1
            (Utilities|FlowControl|DoOnce false :!label _label_3
              (:Completed
                (goto _label_2)))))))
    (:then_2
      (if (== AxisValue 0.0)
        (Utilities|FlowControl|Sequence
          (:then_0
            (goto _label Reset))
          (:then_1
            (goto _label_3 Reset))
          (:then_2
            (Components|Timeline|SetPlayRate (Variables|Default|GetMoveForward) (Variables|Default|GetSpeedWindDown))
            (Timeline|MoveForward Reverse)))))))

(fn ConstructionScript)

(fn IsGrounded
  (return (> (Utilities|Array|Length (Collision|GetOverlappingActors (Variables|Default|GetGroundCheck) 0 :!class /Script/Engine.PrimitiveComponent)) 1)))