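; Basic enemy projectile that fires toward the player when AttackPlayer is called.
; It snaps its yaw to the player, then a speed-scaled timeline lerps it along a fixed straight path while shrinking it, without sweeping.
; Each update polls HitBox overlaps, and any actor lacking the "Entity" tag hides the projectile and disables its collision.
; The actor is destroyed when the timeline finishes; no damage is applied here.
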(event Custom|AttackPlayer
  (params (Player :type BP%20Player%203%20Object%20Reference))
  (bind _returnvalue (Transformation|GetActorLocation))
  (bind _hitbox (Variables|Default|GetHitBox))
  (bind _hitbox_2 (Variables|Default|GetHitBox))
  (bind _overlappingactors (Collision|GetOverlappingActors _hitbox_2 0 :!class /Script/Engine.PrimitiveComponent))
  (Transformation|SetActorRotation (Math|Interpolation|RInterpTo (Transformation|GetActorRotation) (Math|Rotator|MakeRotator 0.0 0.0 (.yaw (Math|Rotator|FindLookatRotation (Transformation|GetActorLocation) (Transformation|GetActorLocation Player)))) (Utilities|Time|GetWorldDeltaSeconds) 0.0))
  (Components|Timeline|SetPlayRate (Variables|Default|GetProjectileTimeline) (Variables|Default|GetProjectileSpeed))
  (Variables|Default|SetStart _returnvalue)
  (Variables|Default|SetFinish (+ _returnvalue (* (Transformation|GetActorForwardVector) (Variables|Default|GetTravelDistance))))
  (Variables|Default|SetStartingScale (Transformation|GetActorScale3D))
  (bind _speed (Timeline|ProjectileTimeline PlayFromStart)
    (:Update
      (Utilities|IsValid _hitbox
        (:Is%20Valid
          (if (> (Utilities|Array|Length _overlappingactors) 0)
            (for _array_element _overlappingactors
              (if (not (Actor|ActorHasTag _array_element "Entity"))
                (Rendering|SetActorHiddenInGame true)
                (Collision|SetCollisionEnabled (Variables|Default|GetHitBox) "NoCollision"))))
          (Transformation|SetActorLocation (Math|Vector|Lerp(Vector) (Variables|Default|GetStart) (Variables|Default|GetFinish) _speed) false false)
          (Transformation|SetActorScale3D (Math|Vector|Lerp(Vector) (Variables|Default|GetStartingScale) (/ (Variables|Default|GetStartingScale) 7.0) _speed)))))
    (:Finished
      (Utilities|IsValid _hitbox
        (:Is%20Valid
          (Actor|DestroyActor))))))

(fn ConstructionScript)