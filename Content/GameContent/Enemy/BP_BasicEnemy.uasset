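; BP_BasicEnemy is a stationary-logic enemy that fires BP_BasicProjectile at the player and is destroyed by a single TakeDamage call.
; Each tick it smoothly yaws toward the BP_Player3 found at BeginPlay and, within SightRange, spawns a projectile through a DoOnce gate.
; A timeline with a randomized play rate serves as the cooldown that resets the gate.
; A visibility trace runs before firing, but its result is unused.
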(event Custom|StartProjectileCoolDown
  (bind _projectilecooldownrange (Variables|Default|GetProjectileCooldownRange))
  (bind _output_get (Variables|Default|SetRandomCooldownRange (Math|Random|RandomFloatinRange _projectilecooldownrange (+ _projectilecooldownrange 2.0))))
  (Components|Timeline|SetPlayRate (Variables|Default|GetEndProjectileTimeline) (/ 1.0 _output_get))
  (bind _speed (Timeline|EndProjectileTimeline PlayFromStart)
    (:Finished
      (Utilities|FlowControl|DoOnce false) ; enters at Reset
    )))

(event EventBeginPlay
  (bind _returnvalue (Actor|GetActorOfClass "/Game/GameContent/Player/BP_Player3.BP_Player3_C"))
  (Variables|Default|SetPlayer _returnvalue))

(event Collision|EventActorBeginOverlap
  (params (OtherActor :type Actor%20Object%20Reference)))

(event EventTick
  (params (DeltaSeconds :type Float%20%28single-precision%29))
  (Utilities|FlowControl|Sequence
    (:then_0
      (Utilities|IsValid (Variables|Default|GetPlayer)
        (:Is%20Valid
          (bind _vectorlength (CallFunction|Magnitude self (Variables|Default|GetPlayer)))
          (if (< _vectorlength (Variables|Default|GetSightRange)) ; If they are in sight range
            (Utilities|FlowControl|DoOnce false
              (:Completed
                (bind _outhit (Collision|LineTraceByChannel (Transformation|GetActorLocation self) (Transformation|GetActorLocation (Variables|Default|GetPlayer)) "TraceTypeQuery1" false 0 "None"))
                (bind _returnvalue (Game|SpawnActorfromClass "/Game/GameContent/Enemy/BP_BasicProjectile.BP_BasicProjectile_C" (Transformation|GetWorldTransform (Variables|Default|GetProjectileSpawnLocation)) "Undefined" 0 0))
                (Default|AttackPlayer _returnvalue (Variables|Default|GetPlayer))
                (CallFunction|StartProjectileCoolDown)))))))
    (:then_1
      (Utilities|IsValid (Variables|Default|GetPlayer)
        (:Is%20Valid
          (Transformation|SetActorRotation (Math|Interpolation|RInterpTo (Transformation|GetActorRotation) (Math|Rotator|MakeRotator 0.0 0.0 (.yaw (Math|Rotator|FindLookatRotation (Transformation|GetActorLocation) (Transformation|GetActorLocation (Variables|Default|GetPlayer))))) (Utilities|Time|GetWorldDeltaSeconds) 5.0)))))))

(event EventTakeDamage
  (Actor|DestroyActor))

(fn ConstructionScript)

(fn Magnitude
  (params (From :type Actor%20Object%20Reference) (To :type Actor%20Object%20Reference))
  (return (Math|Vector|VectorLength (- (Transformation|GetActorLocation From) (Transformation|GetActorLocation To)))))